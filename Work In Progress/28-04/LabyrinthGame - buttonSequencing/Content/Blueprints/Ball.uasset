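; Ball actor that tracks a three-button gate sequence through its overlap events.
; Each overlap casts the other actor to the gate button types and sets a matching flag, checking that the earlier buttons were already hit.
; Pressing button 2 or 3 out of order clears all flags and plays a failure sound.
; Completing the order plays a delayed success sound and sets ComboTrue.
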(event `self.ReceiveActorBeginOverlap`
  (params (OtherActor :type "Actor Object Reference"))
  ;[1 1 1] Checks if the ball is overlapping with a button and sets the corresponding boolean to true if it is.
  (cast `/Game/Blueprints/gateButton1` OtherActor
    (:`then`
      (set `self.isOverlappingButton1` true)
      (`KismetSystemLibrary.PrintString` "Button 1 Pressed")
      (`GameplayStatics.PlaySound2D` "/Game/Assets/Sounds/SFX/buttonPressInGame.buttonPressInGame"))
    (:`CastFailed`
      (cast `/Game/Blueprints/gateButton2` OtherActor
        (:`then`
          (set `self.IsOverlappingButton2` true)
          (`KismetSystemLibrary.PrintString` "Button 2 Pressed")
          (if (`self.isOverlappingButton1`)
            (if (`self.IsOverlappingButton2`)
              (`GameplayStatics.PlaySound2D` "/Game/Assets/Sounds/SFX/buttonPressInGame.buttonPressInGame")
              (else
                (set `self.isOverlappingButton1` false :!label _label)
                (set `self.IsOverlappingButton2` false)
                (set `self.IsOverlappingButton3` false)
                (`GameplayStatics.PlaySound2D` "/Game/Assets/Sounds/SFX/sequenceFailed1.sequenceFailed1" 1.5)))
            (else
              (goto _label))))
        (:`CastFailed`
          (cast `/Game/Blueprints/gateButton3` OtherActor)
          (set `self.IsOverlappingButton3` true)
          (`KismetSystemLibrary.PrintString` "Button 3 Pressed")
          (if (`self.isOverlappingButton1`)
            (if (`self.IsOverlappingButton2`)
              (if (`self.IsOverlappingButton3`)
                (`GameplayStatics.PlaySound2D` "/Game/Assets/Sounds/SFX/buttonPressInGame.buttonPressInGame")
                (`KismetSystemLibrary.Delay` 1.0)
                (`GameplayStatics.PlaySound2D` "/Game/Assets/Sounds/SFX/sequenceCorrect.sequenceCorrect")
                (`KismetSystemLibrary.PrintString` "combo true")
                (set `self.comboTrue` true)
                (else
                  (goto _label)))
              (else
                (goto _label)))
            (else
              (goto _label))))))))

(fn `UserConstructionScript`)