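; Gate Blueprint that slides its cube open once the Ball's ComboTrue flag is set.
; Each Tick it finds the first Ball actor via GetAllActorsOfClass and polls that flag, rather than receiving an event.
; When the flag is true, it plays a timeline that lerps the cube's relative location from GateStart to GateEnd.
; The Box overlap event only casts to Ball and is a leftover test.
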(event `self.Box.OnComponentBeginOverlap`
  (params (OverlappedComponent :type "PrimitiveComponent Object Reference") (OtherActor :type "Actor Object Reference") (OtherComp :type "PrimitiveComponent Object Reference") (OtherBodyIndex :type Integer) (bFromSweep :type Boolean) (SweepResult :type "HitResult Structure (by ref)"))
  ;[1 1 1] ignore - used to check if gate worked before wiring up button
  (cast `/Game/Blueprints/Ball` OtherActor))

(event `self.ReceiveTick`
  (params (DeltaSeconds :type "Float (single-precision)"))
  ;[1 1 1] Every tick, check whether the "Is Overlapping Gate Button" boolean (from gateButton class) is true, if so then run timeline to move the gate
  (bind _outactors (`GameplayStatics.GetAllActorsOfClass` "/Game/Blueprints/Ball.Ball_C")) ; Choosing the actor that is called
  (bind _asball (cast `/Game/Blueprints/Ball` (`|GetArrayItem` _outactors)))
  (if (`/Game/Blueprints/Ball.comboTrue` _asball)
    (bind (_direction _gatemotion) (`Timeline|Timeline - gateAnim`)
      (:`Update`
        (`SceneComponent.K2_SetRelativeLocation` (`self.Cube`) (`KismetMathLibrary.VLerp` (`self.gateStart`) (`self.gateEnd`) _gatemotion) false false)))))

(fn `UserConstructionScript`)