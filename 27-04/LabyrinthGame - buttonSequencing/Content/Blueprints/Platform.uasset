(event `InputAxis|MoveUpDown` :consume false
  (params (AxisValue :type "Float (single-precision)"))
  ;[1 1 1] Ignore
)

(event `InputAxis|MoveLeftRight` :consume false
  (params (AxisValue :type "Float (single-precision)"))
  ;[1 1 1] Ignore
  (`self.K2_SetActorRelativeRotation` (`KismetMathLibrary.MakeRotator` (+ AxisValue (.roll (`self.K2_GetActorRotation`))) (.pitch (`self.K2_GetActorRotation`)) (.yaw (`self.K2_GetActorRotation`)))))

(event `self.ReceiveBeginPlay`
  (bind _returnvalue (`|CreateWidget` "/Game/Blueprints/MyHUD.MyHUD_C"))
  (`UserWidget.AddToViewport` _returnvalue 0))

(event `self.DeathVolume.OnComponentBeginOverlap`
  (params (OverlappedComponent :type "PrimitiveComponent Object Reference") (OtherActor :type "Actor Object Reference") (OtherComp :type "PrimitiveComponent Object Reference") (OtherBodyIndex :type Integer) (bFromSweep :type Boolean) (SweepResult :type "HitResult Structure (by ref)"))
  (cast `/Game/Blueprints/Ball` OtherActor)
  (`KismetSystemLibrary.PrintString` "You died" true true (struct :`R` 1.0 :`G` 0.005986 :`B` 0.864302 :`A` 1.0)))

(fn `UserConstructionScript`)